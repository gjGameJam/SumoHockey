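; BP_SumoPowerUpSpot is a spawn point that respawns a BP_SumoBoost pickup at its own transform after a recharge cooldown.
; TakePowerUp marks the spot empty, after which Tick accumulates time through GetPercentFull, a clamped zero-to-one recharge fraction.
; When that fraction reaches full, the spot spawns a new boost owned by itself, clears the empty flag and resets the timer.
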(event EventBeginPlay)

(event Collision|EventActorBeginOverlap
  (params (OtherActor :type Actor%20Object%20Reference)))

(event EventTick
  (params (DeltaSeconds :type Float%20%28single-precision%29))
  (if (Variables|Default|GetIsEmpty)
    (bind _percentcharge (CallFunction|GetPercentFull DeltaSeconds))
    (Math|Float|CompareFloat _percentcharge 1.0
      (:>
        _)
      (:==
        _))
    (CallFunction|SpawnSumoPowerUp)
    (Variables|Default|SetIsEmpty false)
    (Variables|Default|SetCurrentTime 0.0)))

(fn ConstructionScript)

(fn SpawnSumoPowerUp
  (Game|SpawnActorfromClass "/Game/Blueprints/BP_SumoBoost.BP_SumoBoost_C" (Transformation|GetActorTransform) "Undefined" "MultiplyWithRoot" self 0))

(fn GetPercentFull
  (params (deltaTime :type Float%20%28double-precision%29))
  ;[0.15 0.15 0.15 0.5] Adds delta time to current time charge, divides by cooldown time, and returns 0 - 100 percent (use for recharge icon in game)
  (bind _output_get (Variables|Default|SetCurrentTime (+ (Variables|Default|GetCurrentTime) deltaTime)))
  (return (Math|Float|Clamp(Float) (/ _output_get (Variables|Default|GetTotalRechargeTime)))))

(fn TakePowerUp
  ;[0.15 0.15 0.15 0.5] Power spot is empty, recharge now
  (Variables|Default|SetIsEmpty true))