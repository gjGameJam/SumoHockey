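; BP_SumoBoost is a sumo power-up pickup that grants the boost to a BP_Paddle0 that touches it.
; It plays a spawn sound on BeginPlay and listens for overlaps on its sphere.
; A paddle without the power-up gets its HasSumoPowerUp flag set, then the pickup notifies its owning BP_SumoPowerUpSpot and destroys itself.
; Paddles already holding the power-up only trigger a debug print, and the TakeSumoBoost function is empty.
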(event OnComponentBeginOverlap(Sphere1)
  (params (OverlappedComponent :type Primitive%20Component%20Object%20Reference) (OtherActor :type Actor%20Object%20Reference) (OtherComp :type Primitive%20Component%20Object%20Reference) (OtherBodyIndex :type Integer) (bFromSweep :type Boolean) (SweepResult :type Hit%20Result%20Structure%20%28by%20ref%29))
  (bind _asbp_paddle (Utilities|Casting|CastToBP_Paddle0 OtherActor))
  (if (Variables|/Game/Blueprints/BP_Paddle0.BP_Paddle0_C|GetHasSumoPowerUp _asbp_paddle)
    (Development|PrintString "already has sumo powerup")
    (else
      ;[0.15 0.15 0.15 0.5] Set has sumo power up to true, communicate to spawner that power up was taken, and destroy power up
      (Variables|/Game/Blueprints/BP_Paddle0.BP_Paddle0_C|SetHasSumoPowerUp _asbp_paddle true)
      (bind _asbp_sumo_power_up_spot (Utilities|Casting|CastToBP_SumoPowerUpSpot (Components|GetOwner)))
      (Default|TakePowerUp _asbp_sumo_power_up_spot)
      (Development|PrintString "take")
      (Actor|DestroyActor))))

(event EventBeginPlay
  (Audio|Components|Audio|Play (Variables|Default|GetPOWER_UP_SPAWN_bip_2) 0.0))

(event Collision|EventActorBeginOverlap
  (params (OtherActor :type Actor%20Object%20Reference)))

(event EventTick
  (params (DeltaSeconds :type Float%20%28single-precision%29)))

(fn ConstructionScript)

(fn TakeSumoBoost)