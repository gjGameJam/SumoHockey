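; Goal line actor for a sumo hockey game that scores when a puck enters its box.
; On overlap it destroys the puck, adds a point to the opposing side's scoreboard widget based on GoalID, and plays GOAL.
; BeginPlay caches the drop point transform and both score widgets.
; A new puck spawns there after any overlap, even non-puck ones; the defense sumo check is a stub returning true.
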(event OnComponentBeginOverlap(Box)
  (params (OverlappedComponent :type Primitive%20Component%20Object%20Reference) (OtherActor :type Actor%20Object%20Reference) (OtherComp :type Primitive%20Component%20Object%20Reference) (OtherBodyIndex :type Integer) (bFromSweep :type Boolean) (SweepResult :type Hit%20Result%20Structure%20%28by%20ref%29))
  ;[0.15 0.15 0.15 0.5] If goal line is touched by a puck object, destroy the puck, change the score for correct player, and respawn puck
  (Utilities|FlowControl|Sequence
    (:then_0
      (bind _asbp_puck (Utilities|Casting|CastToBP_Puck OtherActor))
      (Actor|DestroyActor _asbp_puck)
      (switch Utilities|FlowControl|Switch|SwitchonE_GoalTypes (Variables|Default|GetGoalID)
        (:NewEnumerator0
          (Development|PrintString "goal on black!!!")
          (Math|Integer|IncrementInt (Variables|/Game/Blueprints/Widgets/WBP_ScoreWidget.WBP_ScoreWidget_C|GetPoints (Variables|Default|GetWhiteGoalWidg))
            (:%20%20
              _)))
        (:NewEnumerator1
          (Development|PrintString "goal on white!!!")
          (Math|Integer|IncrementInt (Variables|/Game/Blueprints/Widgets/WBP_ScoreWidget.WBP_ScoreWidget_C|GetPoints (Variables|Default|GetBlackGoalWidg))
            (:%20%20
              _))))
      (Audio|Components|Audio|Play (Variables|Default|GetGOAL) 0.0))
    (:then_1
      (CallFunction|RespawnPuck))))

(event EventBeginPlay
  ;[0.15 0.15 0.15 0.5] On start save the puck respawn point to place puck
  (bind _returnvalue (Actor|GetActorOfClass "/Game/Blueprints/BP_PuckDropPoint.BP_PuckDropPoint_C"))
  (Variables|Default|SetPuckSpawnPoint (Transformation|GetActorTransform _returnvalue))
  (bind _returnvalue_2 (Actor|GetActorOfClass "/Game/Blueprints/BP_SumoHockey.BP_SumoHockey_C"))
  (Variables|Default|SetSockeyGameMode _returnvalue_2)
  (CallFunction|GetCorrectScoreWidget))

(event Collision|EventActorBeginOverlap
  (params (OtherActor :type Actor%20Object%20Reference)))

(event EventTick
  (params (DeltaSeconds :type Float%20%28single-precision%29)))

(fn ConstructionScript)

(fn RespawnPuck
  (Game|SpawnActorfromClass "/Game/Blueprints/BP_Puck.BP_Puck_C" (Variables|Default|GetPuckSpawnPoint) "Undefined" "MultiplyWithRoot" 0 0))

(fn CheckifDefenseCanSumo
  (Development|PrintString "defense check")
  (return true))

(fn GetCorrectScoreWidget
  ;[0.15 0.15 0.15 0.5] gets
  (bind _returnvalue (Actor|GetActorOfClass "/Game/Blueprints/BP_ScoreBoard.BP_ScoreBoard_C"))
  (Utilities|FlowControl|Sequence
    (:then_0
      (bind _aswbp_score_widget (Utilities|Casting|CastToWBP_ScoreWidget (UserInterface|GetUserWidgetObject (Variables|/Game/Blueprints/BP_ScoreBoard.BP_ScoreBoard_C|GetBlackScore _returnvalue))))
      (Variables|Default|SetBlackGoalWidg _aswbp_score_widget))
    (:then_1
      (bind _aswbp_score_widget_2 (Utilities|Casting|CastToWBP_ScoreWidget (UserInterface|GetUserWidgetObject (Variables|/Game/Blueprints/BP_ScoreBoard.BP_ScoreBoard_C|GetWhiteScore _returnvalue))))
      (Variables|Default|SetWhiteGoalWidg _aswbp_score_widget_2))))