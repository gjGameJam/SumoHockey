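; Camera manager actor that moves itself between a fixed hockey view and a sumo view at the puck.
; Two events drive timelines that lerp its transform: one toward the puck cube's live location plus an offset, keeping hockey rotation and scale, the other from its current spot back to hockey view.
; ZoomToSumoView and ZoomToHockeyView lerp in a for-loop without delays, so they reach their targets within a single frame.
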(event Custom|LerpToSumoView
  (bind _hockeyview (Variables|Default|GetHockeyView))
  ;[0.15 0.15 0.15 0.5] Lerp from hockey view to puck for sumo view
  (bind _returnvalue (Actor|GetActorOfClass "/Game/Blueprints/BP_Puck.BP_Puck_C"))
  (bind _alphalerp (Timeline|LerpTimeline PlayFromStart)
    (:Update
      (Transformation|SetActorTransform (Math|Transform|Lerp(Transform) (Variables|Default|GetHockeyView) (Math|Transform|MakeTransform (+ (Transformation|GetWorldLocation (Variables|/Game/Blueprints/BP_Puck.BP_Puck_C|GetCube _returnvalue)) (Variables|Default|GetSumoViewPositionOffset)) (.rotation _hockeyview) (.scale _hockeyview)) _alphalerp)))))

(event Custom|LerpToHockeyView
  ;[0.15 0.15 0.15 0.5] Returns from current spot to hockey view
  (Variables|Default|SetStartingTransform (Transformation|GetActorTransform))
  (bind _alphalerp (Timeline|Timeline PlayFromStart)
    (:Update
      (Transformation|SetActorTransform (Math|Transform|Lerp(Transform) (Variables|Default|GetStartingTransform) (Variables|Default|GetHockeyView) _alphalerp)))))

(event EventBeginPlay)

(event Collision|EventActorBeginOverlap
  (params (OtherActor :type Actor%20Object%20Reference)))

(event EventTick
  (params (DeltaSeconds :type Float%20%28single-precision%29)))

(fn ConstructionScript)

(fn ZoomtoSumoView
  (Development|PrintString "zooming" true true "(R=0.000000,G=1.000000,B=0.160949,A=1.000000)")
  (bind _returnvalue (Actor|GetActorOfClass "/Game/Blueprints/BP_Puck.BP_Puck_C"))
  (LocalVariables|SetSumoView (Transformation|GetActorTransform _returnvalue))
  (for _index (range 0 100)
    (Transformation|SetActorTransform (Math|Transform|Lerp(Transform) (Variables|Default|GetHockeyView) (LocalVariables|GetSumoView) (* (LocalVariables|GetPercentConversion) _index)))))

(fn ZoomtoHockeyView
  (LocalVariables|SetStartTransform (Transformation|GetActorTransform))
  (for _index (range 0 100)
    (Transformation|SetActorTransform (Math|Transform|Lerp(Transform) (LocalVariables|GetStartTransform) (Variables|Default|GetHockeyView) (* (LocalVariables|GetPercentConversion) _index)))))