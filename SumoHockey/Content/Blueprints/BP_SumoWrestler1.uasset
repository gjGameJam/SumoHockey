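; Player-controlled sumo wrestler pawn for a sumo face-off minigame within a hockey game.
; A timed start turns button hold time into a forward sphere impulse, then presses play push montages and grunts.
; MoveSumos only draws a debug midpoint, as its circling and time-scaled push impulses are disconnected.
; Tick detects falling by Z velocity, then has BP_SumoHockey despawn sumos, repossess paddles and boost the puck along the puck-to-sumo vector.
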(event Custom|SumoChargeOnStart
  ;[0.15 0.15 0.15 0.5] After sumo start delay, provide charge based on held button time
  (Audio|Components|Audio|Play (Variables|Default|GetStartWhistle) 0.0)
  (bind _newparam (CallFunction|GetSumoStartBoost))
  (Development|PrintString (Utilities|String|ToString(Float) _newparam))
  (Variables|Default|SetStartingPhase false)
  (Physics|AddImpulse (Variables|Default|GetSphere) (* (Math|Vector|GetForwardVector (Variables|Default|GetSphere)) (Variables|Default|GetSumoStartBoostScalar) _newparam) "None" true))

(event Input|EnhancedActionEvents|EnhancedInputActionIA_Push
  (params (ActionValue :type Boolean) (ElapsedSeconds :type Float%20%28double-precision%29) (TriggeredSeconds :type Float%20%28double-precision%29) (InputAction :type Input%20Action%20Object%20Reference :default "/Game/Input/Sumo/IA_Push.IA_Push"))
  ;[0.15 0.15 0.15 0.5] TODO: switch input mapping contexts between sumo and hockey
  (Development|PrintString "sumo push"))

(event Input|EnhancedActionEvents|EnhancedInputActionIA_TurnDirection
  (params (ActionValue :type Float%20%28double-precision%29) (ElapsedSeconds :type Float%20%28double-precision%29) (TriggeredSeconds :type Float%20%28double-precision%29) (InputAction :type Input%20Action%20Object%20Reference :default "/Game/Input/Sumo/IA_TurnDirection.IA_TurnDirection"))
  ;[0.15 0.15 0.15 0.5] TODO: switch input mapping contexts between sumo and hockey
  (Development|PrintString "sumo turn"))

(event Input|EnhancedActionEvents|EnhancedInputActionIA_SumoPowerUp
  (params (ActionValue :type Boolean) (ElapsedSeconds :type Float%20%28double-precision%29) (TriggeredSeconds :type Float%20%28double-precision%29) (InputAction :type Input%20Action%20Object%20Reference :default "/Game/Input/Hockey/IA_SumoPowerUp.IA_SumoPowerUp"))
  (bind _sumowrestler (Variables|Default|GetSumoWrestler))
  (:Started
    ;[0.15 0.15 0.15 0.5] Starting mode needs hold down and after sumo mode needs button mash
    (Math|Integer|IncrementInt (Variables|Default|GetClickCheckNum) :!label _label
      (:%20%20
        (if (Variables|Default|GetStartingPhase)
          (Development|PrintString (Utilities|String|ToString(Float) (CallFunction|GetSumoHoldTime)))
          (else
            ;;[0.15 0.15 0.15 0.5] Each push should move this sumo and opposing sumo around mid point (if joystick input) and forward (relative to this sumo)
            (bind _midpoint (CallFunction|GetMidpointBetweenSumos))
            (CallFunction|MoveSumos _midpoint (.x (Input|EnhancedActionValues|GetIA_MovePaddle)))
            (Development|PrintString (Utilities|String|ToString(Vector) _midpoint))
            (if (Variables|Default|GetCanPush)
              (Audio|Components|Audio|Play (Variables|Default|GetGrunt) 0.0)
              (if (Variables|Default|GetPushStep)
                (Animation|Montage|PlayMontage _sumowrestler "/Game/Art/Sumo/PushL.PushL"
                  (:then
                    (Variables|Default|SetCanPush false :!label _label_2)
                    (Variables|Default|SetPushStep (not (Variables|Default|GetPushStep)))
                    (Utilities|FlowControl|Delay 1.0)
                    (Math|Integer|DecrementInt (Variables|Default|GetClickCheckNum)))
                  (:OnCompleted
                    (Variables|Default|SetCanPush true :!label _label_3)))
                (else
                  (Animation|Montage|PlayMontage _sumowrestler "/Game/Art/Sumo/PushL.PushL"
                    (:then
                      (goto _label_2))
                    (:OnCompleted
                      (goto _label_3)))))))))))
  (:Ongoing
    (goto _label)))

(event Input|EnhancedActionEvents|EnhancedInputActionIA_MovePaddle
  (params (ActionValue :type Vector%202D%20Structure) (ElapsedSeconds :type Float%20%28double-precision%29) (TriggeredSeconds :type Float%20%28double-precision%29) (InputAction :type Input%20Action%20Object%20Reference :default "/Game/Input/Hockey/IA_MovePaddle.IA_MovePaddle"))
  ;[0.15 0.15 0.15 0.5] unused because input mapping is not being switched back and forth from hockey and sumo
)

(event EventBeginPlay
  (bind _sumowrestler (Variables|Default|GetSumoWrestler))
  ;[0.15 0.15 0.15 0.5] After sumo start delay, provide charge based on held button time
  (bind _asplayer_controller (Utilities|Casting|CastToPlayerController (Pawn|GetController))
    (:then
      (bind _playerindex (Class|TurnBasedBlueprintLibrary|GetMyPlayerIndex _asplayer_controller))
      (if (not (== _playerindex 0))
        (Rendering|Material|SetMaterial (Variables|Default|GetSumoWrestler) 0 "/Game/Art/Sumo/SumoPlayer2.SumoPlayer2")))
    (:CastFailed
      _))
  (Utilities|Time|SetTimerbyEvent (delegate Custom|SumoChargeOnStart) (Variables|Default|GetSumoStartDelay))
  (Animation|Montage|PlayMontage _sumowrestler "/Game/Art/Sumo/SumoIntroMontage.SumoIntroMontage"
    (:OnCompleted
      (bind _assumo_anim_bp (Utilities|Casting|CastToSumo_AnimBP (Components|SkeletalMesh|GetAnimInstance _sumowrestler)))
      (Variables|/Game/Art/Sumo/Sumo_AnimBP.Sumo_AnimBP_C|SetIsReady _assumo_anim_bp true))))

(event Collision|EventActorBeginOverlap
  (params (OtherActor :type Actor%20Object%20Reference)))

(event EventTick
  (params (DeltaSeconds :type Float%20%28single-precision%29))
  (bind _sphere (Variables|Default|GetSphere))
  ;[0.15 0.15 0.15 0.5] if falling off, get vector relative to puck center to provide impulse, destroy/depossess sumos, zoom back to hockey view, and repossess paddles
  (bind _isfalling (CallFunction|IsFallingOff))
  (if _isfalling
    (bind _assumo_anim_bp (Utilities|Casting|CastToSumo_AnimBP (Components|SkeletalMesh|GetAnimInstance (Variables|Default|GetSumoWrestler))))
    (Variables|/Game/Art/Sumo/Sumo_AnimBP.Sumo_AnimBP_C|SetIsFalling _assumo_anim_bp true)
    (Variables|/Game/Art/Sumo/Sumo_AnimBP.Sumo_AnimBP_C|SetIsReady _assumo_anim_bp false)
    (Class|PrimitiveComponent|SetAllPhysicsLinearVelocity _sphere (* (Transformation|GetActorForwardVector) -0.25) false)
    (Physics|SetEnableGravity _sphere false)
    (Utilities|FlowControl|Delay 0.2)
    (CallFunction|HandleSumoLoss)))

(fn ConstructionScript)

(fn ChangetoHockeyInput
  (bind _returnvalue (Game|GetPlayerController 0))
  (bind _returnvalue_2 (PlayerController|LocalPlayerSubsystems|GetEnhancedInputLocalPlayerSubsystem _returnvalue))
  ;[0.15 0.15 0.15 0.5] remove sumo and add hockey input mapping context
  (Input|RemoveMappingContext _returnvalue_2 "/Game/Input/Sumo/IMC_Sumo.IMC_Sumo" "(bIgnoreAllPressedKeysUntilRelease=True,bForceImmediately=False,bNotifyUserSettings=False)")
  (Input|AddMappingContext _returnvalue_2 "/Game/Input/Hockey/IM_Hockey.IM_Hockey" 0 "(bIgnoreAllPressedKeysUntilRelease=True,bForceImmediately=False,bNotifyUserSettings=False)"))

(fn IsFallingOff
  ;[0.15 0.15 0.15 0.5] if z velocity is negative above a certain threshold, we know the sumo is falling and has lost first
  (bind _returnvalue (Physics|GetPhysicsLinearVelocity (Variables|Default|GetSphere) "None"))
  (Math|Float|CompareFloat (.z _returnvalue) -5e+01
    (:>
      (return false))
    (:==
      _)
    (:<
      _))
  (return true))

(fn GetPuckBoostDirection
  ;[0.15 0.15 0.15 0.5] this is the falling sumo so get vector going from self to puck for boost direction
  (bind _returnvalue (Actor|GetActorOfClass "/Game/Blueprints/BP_Puck.BP_Puck_C"))
  (return (- (Transformation|GetWorldLocation (Variables|Default|GetSphere)) (Transformation|GetWorldLocation (Variables|/Game/Blueprints/BP_Puck.BP_Puck_C|GetCube _returnvalue)))))

(fn HandleSumoLoss
  (if (not (Variables|Default|GetHasLost))
    (Variables|Default|SetHasLost true)
    (bind _sumotopuck (CallFunction|GetPuckBoostDirection))
    (bind _returnvalue (Actor|GetActorOfClass "/Game/Blueprints/BP_SumoHockey.BP_SumoHockey_C"))
    (Default|DespawnSumos _returnvalue)
    (Utilities|FlowControl|Sequence
      (:then_0
        ;[0.15 0.15 0.15 0.5] only give cooldown to sumos triggered by power ups (not goal line defenses) but still need to provide one second for camera lerp to finish
        (if (Variables|Default|GetSpawnedByPowerup)
          (Variables|/Game/Blueprints/BP_SumoHockey.BP_SumoHockey_C|SetEndOfLastSumo _returnvalue (Utilities|Time|GetTimeSeconds))
          (else
            (Development|PrintString "spawned sumo loss")
            (Variables|/Game/Blueprints/BP_SumoHockey.BP_SumoHockey_C|SetEndOfLastSumo _returnvalue (+ (Utilities|Time|GetTimeSeconds) 2.0)))))
      (:then_1
        (Default|RepossessPaddlesandBoostPuck _returnvalue _sumotopuck)
        (Development|PrintString "falling sumo")))))

(fn GetSumoHoldTime
  ;[0.15 0.15 0.15 0.5] gets how long the facepad bottom button has been pressed
  (return (Class|PlayerController|GetInputKeyTimeDown (Game|GetPlayerController (Variables|/Script/Engine.Controller|GetPlayerState (Pawn|GetController))) "Gamepad_FaceButton_Bottom")))

(fn GetSumoStartBoost
  ;[0.15 0.15 0.15 0.5] return 0 if time held is between min and max sumo boost, return time held if else
  (LocalVariables|SetCurrentHoldTime (CallFunction|GetSumoHoldTime))
  (Math|Float|CompareFloat (LocalVariables|GetCurrentHoldTime) (Variables|Default|GetMaxSumoHoldTime)
    (:>
      (return 0.0))
    (:==
      _)
    (:<
      _))
  (Math|Float|CompareFloat (LocalVariables|GetCurrentHoldTime) (Variables|Default|GetMinSumoHoldTime)
    (:>
      _)
    (:==
      _)
    (:<
      (return 0.0)))
  (return (LocalVariables|GetCurrentHoldTime)))

(fn GetMidpointBetweenSumos
  (bind _outactors (Actor|GetAllActorsOfClass "/Game/Blueprints/BP_SumoWrestler0.BP_SumoWrestler0_C"))
  (bind _returnvalue (Class|GameplayStatics|GetActorArrayAverageLocation _outactors))
  (return _returnvalue))

(fn MoveSumos
  (params (midpoint :type Vector) (xInput :type Float%20%28double-precision%29))
  (LocalVariables|SetSideInput xInput)
  (bind _output_get (LocalVariables|Setmiddle midpoint))
  (Rendering|Debug|DrawDebugSphere _output_get 1e+01 12 "(R=1.000000,G=1.000000,B=1.000000,A=1.000000)" 1.0 1.0)
  (bind _outactors (Actor|GetAllActorsOfClass "/Game/Blueprints/BP_SumoWrestler0.BP_SumoWrestler0_C")))

(fn GetMultiplierfromTime
  ;[0.15 0.15 0.15 0.5] every five seconds, increase amount of force by 20%
  (bind _output_get (LocalVariables|SetTimeForceMulti 2.0))
  (Development|PrintString (Utilities|String|ToString(Float) (Math|Float|Power _output_get (/ (Actor|GetGameTimeSinceCreation) 8.0))))
  (return (Math|Float|Power _output_get (/ (Actor|GetGameTimeSinceCreation) 8.0))))