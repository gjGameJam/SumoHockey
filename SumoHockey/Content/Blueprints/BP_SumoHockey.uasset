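; BP_SumoHockey manages player possession for a two-player air-hockey and sumo hybrid, and opens the main menu on BeginPlay.
; SpawnSumosAndPossess spawns two wrestlers at spots supplied by the puck and hands them to both player controllers.
; DespawnSumos lerps the camera to hockey view and destroys the wrestlers.
; RepossessPaddlesAndBoostPuck returns controllers to paddles by array index, re-enables puck physics and applies a scaled directional impulse.
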(event EventBeginPlay
  (bind _returnvalue (Game|GetPlayerController 0))
  (bind _returnvalue_2 (UserInterface|CreateWidget "/Game/Blueprints/Widgets/WBP_MainMenu.WBP_MainMenu_C" _returnvalue))
  (UserInterface|Viewport|AddtoViewport _returnvalue_2 0)
  (Class|CommonActivatableWidget|ActivateWidget _returnvalue_2)
  (Input|SetInputModeGameandUI _returnvalue _returnvalue_2 "DoNotLock" true false)
  (Class|WidgetBlueprintLibrary|SetFocustoGameViewport))

(event EventTick
  (params (DeltaSeconds :type Float%20%28single-precision%29)))

(fn ConstructionScript)

(fn SpawnSumosandPossess
  (bind _returnvalue (Actor|GetActorOfClass "/Game/Blueprints/BP_Puck.BP_Puck_C"))
  (bind (_spotone _spottwo) (Default|GetSumoStartingSpots _returnvalue))
  (bind _returnvalue_2 (Game|SpawnActorfromClass "/Game/Blueprints/BP_SumoWrestler.BP_SumoWrestler_C" _spotone "AdjustIfPossibleButAlwaysSpawn" "MultiplyWithRoot" 0 0))
  (Pawn|Possess (Game|GetPlayerController 0) _returnvalue_2)
  (bind _returnvalue_3 (Game|SpawnActorfromClass "/Game/Blueprints/BP_SumoWrestler.BP_SumoWrestler_C" _spottwo "AdjustIfPossibleButAlwaysSpawn" "MultiplyWithRoot" 0 0))
  (Pawn|Possess (Game|GetPlayerController 1) _returnvalue_3))

(fn DespawnSumos
  (bind _returnvalue (Actor|GetActorOfClass "/Game/Blueprints/BP_CameraManager.BP_CameraManager_C"))
  (Default|LerptoHockeyView _returnvalue)
  (bind _outactors (Actor|GetAllActorsOfClass "/Game/Blueprints/BP_SumoWrestler.BP_SumoWrestler_C"))
  (for _array_element _outactors
    (Actor|DestroyActor _array_element)))

(fn RepossessPaddlesandBoostPuck
  (params (PuckBoostDir :type Vector))
  (LocalVariables|SetPushDirection (Math|Vector|Normalize PuckBoostDir))
  (bind _outactors (Actor|GetAllActorsOfClass "/Game/Blueprints/BP_Paddle.BP_Paddle_C"))
  (for (_array_element _array_index) _outactors
    (Pawn|Possess (Game|GetPlayerController _array_index) _array_element)
    ;[0.15 0.15 0.15 0.5] get puck, reenable physics, and add appropriate impulse
    (bind _returnvalue (Actor|GetActorOfClass "/Game/Blueprints/BP_Puck.BP_Puck_C"))
    (Physics|SetSimulatePhysics (Variables|/Game/Blueprints/BP_Puck.BP_Puck_C|GetCube _returnvalue) true)
    (Physics|AddImpulse (Variables|/Game/Blueprints/BP_Puck.BP_Puck_C|GetCube _returnvalue) (Math|Vector|MakeVector (.x (* (LocalVariables|GetPushDirection) (Variables|Default|GetSumoPuckBoostScalar))) (.y (* (LocalVariables|GetPushDirection) (Variables|Default|GetSumoPuckBoostScalar))) 0.0) "None" true)
    (Development|PrintString (Utilities|String|Append "sumo boost to puck: " ""))))