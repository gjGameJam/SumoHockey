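; BP_Puck is a physics puck that paddles knock around, and it also carries starting spots for two sumo wrestlers.
; On a hit from a BP_Paddle, it records that paddle and applies a velocity-change impulse along the paddle's BoostDirection, scaled by paddle speed and ForceMultiplier.
; GetSumoStartingSpots offsets two start markers by the cube's world transform, using a helper that adds location and scale and combines rotations.
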(event OnComponentHit(Cube)
  (params (HitComponent :type Primitive%20Component%20Object%20Reference) (OtherActor :type Actor%20Object%20Reference) (OtherComp :type Primitive%20Component%20Object%20Reference) (NormalImpulse :type Vector :default "0, 0, 0") (Hit :type Hit%20Result%20Structure%20%28by%20ref%29))
  (bind _asbp_paddle (Utilities|Casting|CastToBP_Paddle OtherActor))
  (Variables|Default|SetLastPlayerToHit _asbp_paddle)
  (CallFunction|PuckCollision))

(event EventBeginPlay)

(event Collision|EventActorBeginOverlap
  (params (OtherActor :type Actor%20Object%20Reference)))

(event EventTick
  (params (DeltaSeconds :type Float%20%28single-precision%29)))

(fn ConstructionScript)

(fn PuckCollision
  (bind _lastplayertohit (Variables|Default|GetLastPlayerToHit))
  ;[0.15 0.15 0.15 0.5] Launch puck in direction of paddle movement multiplied by force multiplier and paddle speed
  (bind _returnvalue (Physics|GetPhysicsLinearVelocity (Variables|/Game/Blueprints/BP_Paddle.BP_Paddle_C|GetCube _lastplayertohit) "None"))
  (Physics|AddImpulse (Variables|Default|GetCube) (* (Math|Vector|VectorLength _returnvalue) (Math|Conversions|ToVector(Vector2D) (Variables|/Game/Blueprints/BP_Paddle.BP_Paddle_C|GetBoostDirection _lastplayertohit)) (Variables|Default|GetForceMultiplier)) "None" true))

(fn GetSumoStartingSpots
  (bind _cube (Variables|Default|GetCube))
  (bind _returnvalue (Transformation|GetWorldTransform _cube))
  ;[0.15 0.15 0.15 0.5] Gets starting line positions for both sumo wrestlers on puck
  (bind _t3 (CallFunction|AddTransforms (Transformation|GetRelativeTransform (Variables|Default|GetSumoStartOne)) _returnvalue))
  (bind _t3_2 (CallFunction|AddTransforms (Transformation|GetRelativeTransform (Variables|Default|GetSumoStartTwo)) _returnvalue))
  (return _t3 _t3_2))

(fn AddTransforms
  (params (T1 :type Transform) (T2 :type Transform))
  (return (Math|Transform|MakeTransform (+ (.location T1) (.location T2)) (Math|Rotator|CombineRotators (.rotation T1) (.rotation T2)) (+ (.scale T1) (.scale T2)))))