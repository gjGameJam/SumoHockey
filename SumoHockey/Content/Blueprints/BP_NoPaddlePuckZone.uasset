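; BP_NoPaddlePuckZone is a box zone actor for a sumo hockey game, made visible at BeginPlay to debug impassable zones.
; When flagged as GoalZone, a puck overlap calls StartSumoMatch on the cached BP_SumoHockey actor, without player action.
; The defender sumo power-up check is a stub that always returns true.
; RespawnPuck spawns a puck at the cached drop point transform but is not called in this graph.
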(event OnComponentBeginOverlap(Box)
  (params (OverlappedComponent :type Primitive%20Component%20Object%20Reference) (OtherActor :type Actor%20Object%20Reference) (OtherComp :type Primitive%20Component%20Object%20Reference) (OtherBodyIndex :type Integer) (bFromSweep :type Boolean) (SweepResult :type Hit%20Result%20Structure%20%28by%20ref%29))
  ;[0.15 0.15 0.15 0.5] if goal zone is overlapped by puck and defending player has sumo power up, start sumo match (not triggered by player action)
  (if (Variables|Default|GetGoalZone)
    (Utilities|Casting|CastToBP_Puck OtherActor)
    (bind _cansumo (CallFunction|CheckifDefenseCanSumo))
    (if _cansumo
      (Default|StartSumoMatch (Variables|Default|GetSockeyGameMode) false))))

(event EventBeginPlay
  ;[0.15 0.15 0.15 0.5] Debug purposes to see impassable zones
  (Development|SetHiddeninGame (Variables|Default|GetBox) false false)
  (bind _returnvalue (Actor|GetActorOfClass "/Game/Blueprints/BP_PuckDropPoint.BP_PuckDropPoint_C"))
  (Variables|Default|SetPuckSpawnPoint (Transformation|GetActorTransform _returnvalue))
  (bind _returnvalue_2 (Actor|GetActorOfClass "/Game/Blueprints/BP_SumoHockey.BP_SumoHockey_C"))
  (Variables|Default|SetSockeyGameMode _returnvalue_2))

(event Collision|EventActorBeginOverlap
  (params (OtherActor :type Actor%20Object%20Reference)))

(event EventTick
  (params (DeltaSeconds :type Float%20%28single-precision%29)))

(fn ConstructionScript)

(fn RespawnPuck
  (Game|SpawnActorfromClass "/Game/Blueprints/BP_Puck.BP_Puck_C" (Variables|Default|GetPuckSpawnPoint) "Undefined" "MultiplyWithRoot" 0 0))

(fn CheckifDefenseCanSumo
  (Development|PrintString "defense check")
  (return true))