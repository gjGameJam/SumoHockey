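; Player-controlled air hockey paddle that can spend a power-up to switch the game into a sumo match.
; Stick input moves it by swept location updates, paused during impulse boosts that draw on two timer-recharged charges.
; The sumo power-up, gated by the game mode's cooldown check, unpossesses both players and starts the match.
; BeginPlay takes the paddle's side from the nearest goal line; Tick refreshes boost and power-up indicator widgets.
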(event Custom|RestoreOneBoost
  ;[0.15 0.15 0.15 0.5] Trigger to boost paddle
  (if (Variables|Default|GetCanFirstBoost)
    (Variables|Default|SetCanSecondBoost true)
    (else
      (Variables|Default|SetCanFirstBoost true))))

(event Input|EnhancedActionEvents|EnhancedInputActionIA_BoostPaddle
  (params (ActionValue :type Boolean) (ElapsedSeconds :type Float%20%28double-precision%29) (TriggeredSeconds :type Float%20%28double-precision%29) (InputAction :type Input%20Action%20Object%20Reference :default "/Game/Input/Hockey/IA_BoostPaddle.IA_BoostPaddle"))
  ;[0.15 0.15 0.15 0.5] Trigger to boost paddle
  (if (Variables|Default|GetCanFirstBoost)
    (Variables|Default|SetCanFirstBoost false)
    (Utilities|Time|SetTimerbyEvent (delegate Custom|RestoreOneBoost) (Variables|Default|GetBoostRecoveryTime) :!label _label)
    (Physics|AddImpulse (Variables|Default|GetCube) (* (Math|Conversions|ToVector(Vector2D) (Variables|Default|GetBoostDirection)) (Variables|Default|GetBoostSpeed)) "None" true)
    (Variables|Default|SetIsBoosting true)
    (Utilities|FlowControl|RetriggerableDelay 0.6)
    (Variables|Default|SetIsBoosting false)
    (elif (Variables|Default|GetCanSecondBoost)
      (Variables|Default|SetCanSecondBoost false)
      (goto _label))))

(event Input|EnhancedActionEvents|EnhancedInputActionIA_MovePaddle
  (params (ActionValue :type Vector%202D%20Structure) (ElapsedSeconds :type Float%20%28double-precision%29) (TriggeredSeconds :type Float%20%28double-precision%29) (InputAction :type Input%20Action%20Object%20Reference :default "/Game/Input/Hockey/IA_MovePaddle.IA_MovePaddle"))
  ;[0.15 0.15 0.15 0.5] Joystick to move paddle
  (CallFunction|MovePaddle (* (.x ActionValue) -1.0) (.y ActionValue)))

(event Input|EnhancedActionEvents|EnhancedInputActionIA_SumoPowerUp
  (params (ActionValue :type Boolean) (ElapsedSeconds :type Float%20%28double-precision%29) (TriggeredSeconds :type Float%20%28double-precision%29) (InputAction :type Input%20Action%20Object%20Reference :default "/Game/Input/Hockey/IA_SumoPowerUp.IA_SumoPowerUp"))
  ;[0.15 0.15 0.15 0.5] Activates sumo power up
  (bind _canstart (Default|CanStartNewSumoMatch (Variables|Default|GetSockeyGameMode)))
  (if (and _canstart (Variables|Default|GetHasSumoPowerUp))
    (Audio|Components|Audio|Play (Variables|Default|GetPowerUpUse) 0.0)
    (Development|PrintString "sumo time")
    (Variables|Default|SetHasSumoPowerUp false)
    ;[0.15 0.15 0.15 0.5] Unpossess paddles, stop all paddles and puck, lerp to sumo view and create sumos
    (Pawn|UnPossess (Game|GetPlayerController 0))
    (Pawn|UnPossess (Game|GetPlayerController 1))
    (Default|StartSumoMatch (Variables|Default|GetSockeyGameMode) true)
    (else
      (Development|PrintString "no sumo powerup or match on cooldown"))))

(event EventBeginPlay
  ;[0.15 0.15 0.15 0.5] Loop to recover boosts
  (CallFunction|SetSideonStart)
  (bind _returnvalue (Actor|GetActorOfClass "/Game/Blueprints/BP_CameraManager.BP_CameraManager_C"))
  (Variables|Default|SetCameraManager _returnvalue)
  (bind _returnvalue_2 (Actor|GetActorOfClass "/Game/Blueprints/BP_SumoHockey.BP_SumoHockey_C"))
  (Variables|Default|SetSockeyGameMode _returnvalue_2))

(event Collision|EventActorBeginOverlap
  (params (OtherActor :type Actor%20Object%20Reference)))

(event EventTick
  (params (DeltaSeconds :type Float%20%28single-precision%29))
  ;[0.15 0.15 0.15 0.5] want to change to have sumo changed on power up collect but for sake of time do here
  (CallFunction|UpdatePowerUpUI))

(fn ConstructionScript)

(fn MovePaddle
  (params (XMove :type Float%20%28double-precision%29) (YMove :type Float%20%28double-precision%29))
  (Variables|Default|SetBoostDirection (Math|Vector2D|MakeVector2D XMove YMove))
  (if (not (Variables|Default|GetIsBoosting))
    (Transformation|SetActorLocation (Math|Vector|MakeVector (.X (Math|Vector|BreakVector (+ (* (Math|Conversions|ToVector(Vector2D) (Variables|Default|GetBoostDirection)) (Variables|Default|GetMoveSpeed) (Utilities|Time|GetWorldDeltaSeconds)) (Transformation|GetActorLocation)))) (.Y (Math|Vector|BreakVector (+ (* (Math|Conversions|ToVector(Vector2D) (Variables|Default|GetBoostDirection)) (Variables|Default|GetMoveSpeed) (Utilities|Time|GetWorldDeltaSeconds)) (Transformation|GetActorLocation)))) 0.0) true false)))

(fn StopAllAirHockeyPieces
  (Utilities|FlowControl|Sequence
    (:then_0
      (bind _outactors (Actor|GetAllActorsOfClass "BP_Paddle0_C"))
      (for _array_element _outactors
        (Physics|SetPhysicsLinearVelocity (Variables|BP_Paddle0_C|GetCube _array_element) "0, 0, 0" false "None")
        (Class|PrimitiveComponent|SetPhysicsAngularVelocityinDegrees (Variables|BP_Paddle0_C|GetCube _array_element) "0, 0, 0" false "None")))
    (:then_1
      (bind _outactors_2 (Actor|GetAllActorsOfClass "/Game/Blueprints/BP_Puck.BP_Puck_C"))
      (for _array_element_2 _outactors_2
        (Physics|SetPhysicsLinearVelocity (Variables|/Game/Blueprints/BP_Puck.BP_Puck_C|GetCube _array_element_2) "0, 0, 0" false "None")
        (Class|PrimitiveComponent|SetPhysicsAngularVelocityinDegrees (Variables|/Game/Blueprints/BP_Puck.BP_Puck_C|GetCube _array_element_2) "0, 0, 0" false "None")
        (Physics|SetSimulatePhysics (Variables|/Game/Blueprints/BP_Puck.BP_Puck_C|GetCube _array_element_2) false)))))

(fn ChangetoSumoInput
  (bind _returnvalue (Game|GetPlayerController 0))
  (bind _returnvalue_2 (PlayerController|LocalPlayerSubsystems|GetEnhancedInputLocalPlayerSubsystem _returnvalue))
  ;[0.15 0.15 0.15 0.5] Removes hockey mapping and adds sumo mapping
  (Input|RemoveMappingContext _returnvalue_2 "/Game/Input/Hockey/IM_Hockey.IM_Hockey" "(bIgnoreAllPressedKeysUntilRelease=True,bForceImmediately=False,bNotifyUserSettings=False)")
  (Input|AddMappingContext _returnvalue_2 "/Game/Input/Sumo/IMC_Sumo.IMC_Sumo" 0 "(bIgnoreAllPressedKeysUntilRelease=True,bForceImmediately=False,bNotifyUserSettings=False)"))

(fn SetSideonStart
  ;[0.15 0.15 0.15 0.5] sets the first paddle to the type of the goal that they spawn next to and other paddle to opposite of first
  (bind _outactors (Actor|GetAllActorsOfClass "/Game/Blueprints/BP_GoalLine.BP_GoalLine_C"))
  (for _array_element _outactors
    (Math|Float|CompareFloat (Math|Vector|VectorLength (- (Transformation|GetActorLocation _array_element) (Transformation|GetActorLocation))) (LocalVariables|GetShortestDist)
      (:==
        _)
      (:<
        _))
    (LocalVariables|SetShortestDist (Math|Vector|VectorLength (- (Transformation|GetActorLocation _array_element) (Transformation|GetActorLocation))))
    (Variables|Default|SetPaddleType (Variables|/Game/Blueprints/BP_GoalLine.BP_GoalLine_C|GetGoalID _array_element)))
  (Development|PrintString (Utilities|String|EnumtoString (Variables|Default|GetPaddleType))))

(fn UpdatePowerUpUI
  ;[0.15 0.15 0.15 0.5] check if paddle has power up and set UI element accordingly
  (Utilities|FlowControl|Sequence
    (:then_0
      (bind _aswbp_paddle_boost_indicator (Utilities|Casting|CastToWBP_PaddleBoostIndicator (UserInterface|GetWidget (Variables|Default|GetFirstBoostIndicator))))
      (if (Variables|Default|GetCanFirstBoost)
        (Default|Seton _aswbp_paddle_boost_indicator)
        (else
          (Default|SetOff _aswbp_paddle_boost_indicator))))
    (:then_1
      (bind _aswbp_paddle_boost_indicator_2 (Utilities|Casting|CastToWBP_PaddleBoostIndicator (UserInterface|GetWidget (Variables|Default|GetSecondBoostIndicator))))
      (if (Variables|Default|GetCanSecondBoost)
        (Default|Seton _aswbp_paddle_boost_indicator_2)
        (else
          (Default|SetOff _aswbp_paddle_boost_indicator_2))))
    (:then_2
      (bind _aswbp_paddle_sumo_indicator (Utilities|Casting|CastToWBP_PaddleSumoIndicator (UserInterface|GetWidget (Variables|Default|GetSumoBoostIndicator))))
      (if (Variables|Default|GetHasSumoPowerUp)
        (Default|Seton _aswbp_paddle_sumo_indicator)
        (else
          (Default|SetOff _aswbp_paddle_sumo_indicator))))))